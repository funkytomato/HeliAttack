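; Base Blueprint for damageable structures that switch to a destroyed mesh.
; AnyDamage forwards the damage to MasterDamageComponentBP, along with the critical damage value read by casting the damage causer to BP_MasterProjectile.
; If IsDestroyed is true afterwards, a DoOnce swaps the static mesh to DestroyedMesh a single time.
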(event `self.ReceiveAnyDamage`
  (params (Damage :type "Float (single-precision)") (DamageType :type "DamageType Object Reference") (InstigatedBy :type "Controller Object Reference") (DamageCauser :type "Actor Object Reference"))
  (`/Game/MyContent/Blueprints/HelicopterComponents/MasterDamageComponent_BP.ReceiveDamage` (`self.MasterDamageComponent_BP`) self Damage (`/Game/ArcadeHelicopter/Blueprints/BP_MasterProjectile.CriticalDamage` (cast `/Game/ArcadeHelicopter/Blueprints/BP_MasterProjectile` DamageCauser :!pure true)))
  (if (`self.IsDestroyed`)
    (`/Engine/EditorBlueprintResources/StandardMacros.DoOnce` false
      (:`Completed`
        (`StaticMeshComponent.SetStaticMesh` (`self.StaticMesh`) (`self.DestroyedMesh`))))))

(fn `UserConstructionScript`)