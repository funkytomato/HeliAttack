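; Player controller for a top-down helicopter game that turns input into flight and weapon commands for the pawn.
; While flying in Top Down Free mode, Tick applies movement and smoothly rotates the heli toward the cursor or face-axis input, banking it with movement.
; It also derives PitchAngle for rocket pods and, on some rotation paths, DeltaRot for the rotor.
; Weapon selection, trigger and homing-target inputs go to the pawn as messages; IsDead always returns false.
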(fn `IsDead?`
  (returns (`Y/N` :type Boolean))
  (return false))

(fn `MoveToHitLocation`
  (params (Hit :type "HitResult Structure"))
  (bind (_bblockinghit _binitialoverlap _time _distance _location) (`GameplayStatics.BreakHitResult` Hit))
  (if (>= (`KismetMathLibrary.VSize` (- (`self.K2_GetActorLocation` (`self.K2_GetPawn`)) _location)) (`self.MinClickDistance`))
    (`Pawn.AddMovementInput` (`GameplayStatics.GetPlayerPawn` 0) (`KismetMathLibrary.MakeVector` (.x _location) (.y _location)) (`KismetMathLibrary.Conv_BoolToDouble` (or (`KismetInputLibrary.PointerEvent_IsMouseButtonDown` (make `PointerEvent`) "RightMouseButton") (`.bIsCurrentlyPressed` (`self.GetInputTouchState` "Touch1")))) false)
    (`Pawn.AddMovementInput` (`self.K2_GetPawn`) (`KismetMathLibrary.MakeVector` (.x _location) (.y _location)) (`KismetMathLibrary.Conv_BoolToDouble` (or (`KismetInputLibrary.PointerEvent_IsMouseButtonDown` (make `PointerEvent`) "RightMouseButton") (`.bIsCurrentlyPressed` (`self.GetInputTouchState` "Touch1")))) false)
    (return)))

(fn `UserConstructionScript`)