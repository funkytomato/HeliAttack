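; Sniper02_BP is a sniper gun Blueprint that fires projectiles repeatedly while shooting is active.
; StartShooting calls the parent logic, fires once immediately, then starts a looping timer that calls FireProjectile by name at the FireRate interval.
; StopShooting calls the parent logic and clears that timer through its stored handle.
; FireProjectile is not defined in this graph, and the construction script only calls its parent.
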(event `self.StartShooting`
  (`parent.StartShooting`)
  (`self.FireProjectile`)
  (bind _returnvalue (`KismetSystemLibrary.K2_SetTimer` null "FireProjectile" (`self.FireRate`) true))
  (set `self.FireProjectileTimer` _returnvalue))

(event `self.StopShooting`
  (`parent.StopShooting`)
  (`KismetSystemLibrary.K2_ClearAndInvalidateTimerHandle` (`self.FireProjectileTimer`)))

(fn `UserConstructionScript`
  (`parent.UserConstructionScript`))