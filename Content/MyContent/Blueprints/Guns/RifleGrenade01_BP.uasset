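; Rifle with grenade launcher Blueprint that extends a parent gun class with timed automatic firing.
; StartShooting and LaunchGrenade both fire FireProjectile immediately, then loop it on a timer at their respective fire rates until StopShooting clears it.
; A separate FireGrenade function, not called by these events, spawns a HydraRocket projectile at the launcher point, aimed along the parent character's follow camera.
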(event `self.StartShooting`
  (`parent.StartShooting`)
  (`self.FireProjectile`)
  (bind _returnvalue (`KismetSystemLibrary.K2_SetTimer` null "FireProjectile" (`self.FireRate`) true))
  (set `self.FireProjectileTimer` _returnvalue))

(event `LaunchGrenade`
  (`self.FireProjectile`)
  (bind _returnvalue (`KismetSystemLibrary.K2_SetTimer` null "FireProjectile" (`self.GrenadeFireRate`) true))
  (set `self.FireProjectileTimer` _returnvalue))

(event `self.StopShooting`
  (`parent.StopShooting`)
  (`KismetSystemLibrary.K2_ClearAndInvalidateTimerHandle` (`self.FireProjectileTimer`)))

(fn `FireGrenade`
  (bind _assynty_character_bp (cast `/Game/MyContent/Blueprints/Soldiers/Synty_Character_BP` (`self.GetParentActor`)))
  (`|SpawnActorFromClass` "/Game/MyContent/Blueprints/Projectiles/Projectile_HydraRocket_BP.Projectile_HydraRocket_BP_C" (`KismetMathLibrary.MakeTransform` (`SceneComponent.K2_GetComponentLocation` (`self.Launcher_RfPt`)) (`SceneComponent.K2_GetComponentRotation` (`/Game/MyContent/Blueprints/Soldiers/Synty_Character_BP.FollowCamera` _assynty_character_bp))) "AlwaysSpawn" "OverrideRootScale" null 3000.0 3000.0 false 0.0 false null null))

(fn `UserConstructionScript`
  (`parent.UserConstructionScript`))