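; GunMaster_BP is a gun actor that fires projectiles for its parent Synty_Character_BP.
; Construction snaps GunMesh to the root component.
; FireProjectile spawns TestProjectile_BP at the muzzle reference point, rotated to the character's follow camera, with a fixed speed.
; StartShooting and StopShooting both set IsFiring to true, nothing here calls FireProjectile, and an arms montage call is left unconnected.
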(event `StartShooting`
  (set `self.IsFiring` true))

(event `StopShooting`
  (set `self.IsFiring` true))

(fn `FireProjectile`
  (bind _assynty_character_bp (cast `/Game/MyContent/Blueprints/Soldiers/Synty_Character_BP` (`self.GetParentActor`)))
  (`|SpawnActorFromClass` "/Game/MyContent/Blueprints/Projectiles/TestProjectile_BP.TestProjectile_BP_C" (`KismetMathLibrary.MakeTransform` (`SceneComponent.K2_GetComponentLocation` (`self.Muzzle_RfPt`)) (`SceneComponent.K2_GetComponentRotation` (`/Game/MyContent/Blueprints/Soldiers/Synty_Character_BP.FollowCamera` _assynty_character_bp))) "AlwaysSpawn" "OverrideRootScale" null 5000.0 5000.0 false 0.0 false null null))

(fn `UserConstructionScript`
  (`SceneComponent.K2_AttachToComponent` (`self.GunMesh`) (`self.DefaultSceneRoot`) "None" "SnapToTarget" "SnapToTarget" "SnapToTarget" true))