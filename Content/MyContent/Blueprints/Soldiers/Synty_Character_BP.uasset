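; Soldier character Blueprint that tracks health, ammo and combat state, with placeholder attack logic that only prints a message.
; Dispatchers bound on BeginPlay route boosts, drains and attack orders to handlers that clamp values and update low-resource flags; damage also drains health.
; An influence sphere sets CanAttack while the helicopter is in range and briefly flags UnderFire on projectile overlap.
; Both decrease handlers compute amount minus current value, reversing the expected subtraction.
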(event `self.ReceiveBeginPlay`
  ;[1 1 1] Beginplay, assign messages
  (`self.AssignMessages`))

(event `AssignMessages`
  ;[1 1 1] Assign Event Dispatch Messages
  (add `self.HealthBoost` (delegate `HealthBoost_Event`))
  (add `self.HealthDrain` (delegate `HealthDrain_Event`))
  (add `self.AmmoBoost` (delegate `AmmoBoost_Event`))
  (add `self.AmmoDrain` (delegate `AmmoDrain_Event`))
  (add `self.AttackTarget` (delegate `AttackTarget_Event`)))

(event `HealthBoost_Event` :!signature `self.HealthBoost`
  (params (Amount :type "Float (double-precision)"))
  ;[1 1 1] Assign Event Dispatch Messages
  (`self.IncreaseHealth` Amount))

(event `HealthDrain_Event` :!signature `self.HealthDrain`
  (params (Amount :type "Float (double-precision)"))
  ;[1 1 1] Assign Event Dispatch Messages
  (`self.DecreaseHealth` Amount))

(event `AmmoBoost_Event` :!signature `self.AmmoBoost`
  (params (Amount :type "Float (double-precision)"))
  ;[1 1 1] Assign Event Dispatch Messages
  (`self.IncreaseAmmo` Amount))

(event `AmmoDrain_Event` :!signature `self.AmmoDrain`
  (params (Amount :type "Float (double-precision)"))
  ;[1 1 1] Assign Event Dispatch Messages
  (`self.DecreaseAmmo` Amount))

(event `AttackTarget_Event` :!signature `self.AttackTarget`
  (params (Target :type "Actor Object Reference"))
  ;[1 1 1] Assign Event Dispatch Messages
  (`self.Attack` Target))

(event `self.AttackInfluenceSphere.OnComponentBeginOverlap`
  (params (OverlappedComponent :type "PrimitiveComponent Object Reference") (OtherActor :type "Actor Object Reference") (OtherComp :type "PrimitiveComponent Object Reference") (OtherBodyIndex :type Integer) (bFromSweep :type Boolean) (SweepResult :type "HitResult Structure (by ref)"))
  ;[1 1 1] Player within proximity, attack
  (cast `/Game/MyContent/Blueprints/Player/MasterHeli_BP` OtherActor
    (:`then`
      (set `self.CanAttack` true))
    (:`CastFailed`
      ;[1 1 1] Recieving Incoming Fire
      (cast `/Game/MyContent/Blueprints/Projectiles/MasterProjectile_BP` OtherActor)
      (set `self.UnderFire` true)
      (`KismetSystemLibrary.Delay` 1.0)
      (set `self.UnderFire` false))))

(event `Attack`
  (params (Target :type "Actor Object Reference"))
  ;[1 1 1] Attack Target
  (`KismetSystemLibrary.PrintString` "Attacking:")
  (`KismetSystemLibrary.PrintString` "Attacking:"))

(event `self.AttackInfluenceSphere.OnComponentEndOverlap`
  (params (OverlappedComponent :type "PrimitiveComponent Object Reference") (OtherActor :type "Actor Object Reference") (OtherComp :type "PrimitiveComponent Object Reference") (OtherBodyIndex :type Integer))
  ;[1 1 1] Player has gone out of range
  (cast `/Game/MyContent/Blueprints/Player/MasterHeli_BP` OtherActor)
  (set `self.CanAttack` false))

(event `DecreaseHealth`
  (params (amount :type "Float (double-precision)"))
  ;[1 1 1] Decrease health, and set HasLOwHealth respectivily
  (bind _output_get (set `self.Health` (`KismetMathLibrary.FClamp` (- amount (`self.Health`)) 0.0 100.0)))
  (set `self.HasLowHealth` (< _output_get (`self.LowHealthValue`))))

(event `IncreaseHealth`
  (params (Amount :type "Float (double-precision)"))
  ;[1 1 1] Increase Health, and set LowHealth respectivily
  (bind _output_get (set `self.Health` (`KismetMathLibrary.FClamp` (+ Amount (`self.Health`)) 0.0 100.0)))
  (set `self.HasLowHealth` (< _output_get (`self.LowHealthValue`))))

(event `DecreaseAmmo`
  (params (Amount :type "Float (double-precision)"))
  ;[1 1 1] Decrease Ammo, and set HasLowAmmo respectivily
  (bind _output_get (set `self.Ammo` (`KismetMathLibrary.FClamp` (- Amount (`self.Ammo`)) 0.0 (`self.MaxAmmo`))))
  (set `self.HasLowAmmo` (< _output_get (`self.LowAmmoValue`)))
  (if (> _output_get 0.0)
    (set `self.HasAmmo` true)
    (else
      (set `self.HasAmmo` false))))

(event `IncreaseAmmo`
  (params (Amount :type "Float (double-precision)"))
  ;[1 1 1] Increase Ammo, and set HasLowAmmo respectivily
  (bind _output_get (set `self.Ammo` (`KismetMathLibrary.FClamp` (+ Amount (`self.Ammo`)) 0.0 (`self.MaxAmmo`))))
  (set `self.HasLowAmmo` (< _output_get (`self.LowAmmoValue`)))
  (if (> _output_get 0.0)
    (set `self.HasAmmo` true)
    (else
      (set `self.HasAmmo` false))))

(event `self.ReceiveAnyDamage`
  (params (Damage :type "Float (single-precision)") (DamageType :type "DamageType Object Reference") (InstigatedBy :type "Controller Object Reference") (DamageCauser :type "Actor Object Reference"))
  ;[1 1 1] Receive AnyDamage, reduce Health
  (`self.DecreaseHealth` Damage))

(fn `UpdateWalkSpeed`
  (params (`Max Walk Speed` :type "Float (double-precision)"))
  (set `CharacterMovementComponent.MaxWalkSpeed` `Max Walk Speed` (`self.CharacterMovement`)))

(fn `UserConstructionScript`)