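; Base Blueprint for destructible structures that take damage and break apart into physics debris.
; AnyDamage passes the damage, plus CriticalDamage from the MasterProjectile_BP causer, to StructureDamageComponent, then enables physics on the DestructibleComponent after a short delay if IsDestroyed.
; On fracture, the component enables gravity, adjusts collision responses and applies a radial force from just above its location.
; The sound and actor-destroy nodes are unconnected and never run.
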(event `self.ReceiveBeginPlay`)

(event `self.DestructibleComponent.OnComponentFracture`
  (params (HitPoint :type "Vector Structure (by ref)") (HitDirection :type "Vector Structure (by ref)"))
  (bind (_returnvalue_x _returnvalue_y _returnvalue_z) (`KismetMathLibrary.BreakVector` (`SceneComponent.K2_GetComponentLocation` (`self.DestructibleComponent`))))
  ;[1 1 1] Set Fracture objects Collision Responder and Make a Sound on destruction
  (`PrimitiveComponent.SetEnableGravity` (`self.DestructibleComponent`) true)
  (`PrimitiveComponent.SetCollisionResponseToChannel` (`self.DestructibleComponent`) "ECC_PhysicsBody" "ECR_Ignore")
  (`PrimitiveComponent.SetCollisionResponseToChannel` (`self.DestructibleComponent`) "ECC_Destructible" "ECR_Block")
  (`PrimitiveComponent.SetCollisionResponseToChannel` (`self.DestructibleComponent`) "ECC_WorldStatic" "ECR_Block")
  (`PrimitiveComponent.AddRadialForce` (`self.DestructibleComponent`) (`KismetMathLibrary.MakeVector` _returnvalue_x _returnvalue_y (+ _returnvalue_z 50.0)) 500.0 100.0 "RIF_Constant" false))

(event `self.ReceiveAnyDamage`
  (params (Damage :type "Float (single-precision)") (DamageType :type "DamageType Object Reference") (InstigatedBy :type "Controller Object Reference") (DamageCauser :type "Actor Object Reference"))
  ;[1 1 1] AnyDamage received, Apply Damage
  (`/Game/MyContent/Blueprints/Components/Damage/MasterDamageComponent_BP.ReceiveDamage` (`self.StructureDamageComponent`) self Damage (`/Game/MyContent/Blueprints/Projectiles/MasterProjectile_BP.CriticalDamage` (cast `/Game/MyContent/Blueprints/Projectiles/MasterProjectile_BP` DamageCauser :!pure true)))
  (if (`self.IsDestroyed`)
    (`KismetSystemLibrary.Delay` 1.0)
    (`PrimitiveComponent.SetSimulatePhysics` (`self.DestructibleComponent`) true)))

(fn `UserConstructionScript`)