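; Base Blueprint for damageable structures that switch from a static to a skeletal mesh when destroyed.
; BeginPlay seeds DamageComponent with health and armor, and AnyDamage forwards damage plus the causing projectile's critical damage to it.
; When IsDestroyed is set, the skeletal mesh is shown with collision enabled, and hits on it call Fracture.
; Fracture only prints a debug string; the destructible impulse, sound and actor cleanup logic is disconnected.
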(event `self.ReceiveBeginPlay`
  (bind _damagecomponent (`self.DamageComponent`))
  (set `/Game/MyContent/Blueprints/Components/Damage/ActorDamageComponent_BP.Health` (`self.StructureHealth`) _damagecomponent)
  (set `/Game/MyContent/Blueprints/Components/Damage/ActorDamageComponent_BP.ArmorPercentage` (`self.StructureArmor`) _damagecomponent))

(event `EnableDestructible`
  (bind _skeletalmesh (`self.SkeletalMesh`))
  (`KismetSystemLibrary.PrintString` "Switching Static to Skeletal")
  (`SceneComponent.SetVisibility` (`self.StaticMesh`) false false)
  (`SceneComponent.SetVisibility` _skeletalmesh true false)
  (`PrimitiveComponent.SetCollisionEnabled` _skeletalmesh "QueryAndPhysics"))

(event `self.ReceiveAnyDamage`
  (params (Damage :type "Float (single-precision)") (DamageType :type "DamageType Object Reference") (InstigatedBy :type "Controller Object Reference") (DamageCauser :type "Actor Object Reference"))
  (`/Game/MyContent/Blueprints/Components/Damage/ActorDamageComponent_BP.ReceiveDamage` (`self.DamageComponent`) self Damage (`/Game/MyContent/Blueprints/Projectiles/MasterProjectile_BP.CriticalDamage` (cast `/Game/MyContent/Blueprints/Projectiles/MasterProjectile_BP` DamageCauser :!pure true)))
  (if (`self.IsDestroyed`)
    (`self.EnableDestructible`)))

(event `self.SkeletalMesh.OnComponentHit`
  (params (HitComponent :type "PrimitiveComponent Object Reference") (OtherActor :type "Actor Object Reference") (OtherComp :type "PrimitiveComponent Object Reference") (NormalImpulse :type "Vector Structure") (Hit :type "HitResult Structure (by ref)"))
  (`KismetSystemLibrary.PrintString` "SkeletalMesh Hit")
  (`self.Fracture`))

(event `Fracture`
  ;[1 1 1] Set Fracture objects Collision Responder and Make a Sound on destruction
  (`KismetSystemLibrary.PrintString` "Fracture"))

(fn `UserConstructionScript`)