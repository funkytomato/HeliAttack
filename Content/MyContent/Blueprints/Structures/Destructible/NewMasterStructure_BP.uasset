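; Base Blueprint for a destructible structure that takes damage and is removed from the game once destroyed.
; On BeginPlay it copies its health and armor settings into a DamageComponent.
; AnyDamage forwards each hit to that component, taking the critical damage value from the causing MasterProjectile_BP.
; Once IsDestroyed is set, a DoOnce adds a destructible component and immediately destroys the actor.
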(event `self.ReceiveBeginPlay`
  (bind _damagecomponent (`self.DamageComponent`))
  (set `/Game/MyContent/Blueprints/Components/Damage/ActorDamageComponent_BP.Health` (`self.StructureHealth`) _damagecomponent)
  (set `/Game/MyContent/Blueprints/Components/Damage/ActorDamageComponent_BP.ArmorPercentage` (`self.StructureArmor`) _damagecomponent))

(event `self.ReceiveAnyDamage`
  (params (Damage :type "Float (single-precision)") (DamageType :type "DamageType Object Reference") (InstigatedBy :type "Controller Object Reference") (DamageCauser :type "Actor Object Reference"))
  (`/Game/MyContent/Blueprints/Components/Damage/ActorDamageComponent_BP.ReceiveDamage` (`self.DamageComponent`) self Damage (`/Game/MyContent/Blueprints/Projectiles/MasterProjectile_BP.CriticalDamage` (cast `/Game/MyContent/Blueprints/Projectiles/MasterProjectile_BP` DamageCauser :!pure true)))
  (if (`self.IsDestroyed`)
    (`/Engine/EditorBlueprintResources/StandardMacros.DoOnce` false
      (:`Completed`
        (`AddComponent|NODE_AddDestructibleComponent-0`)
        (`self.K2_DestroyActor`)))))

(fn `UserConstructionScript`)