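; Base pawn for destructible structures that take projectile damage and break apart when destroyed.
; BeginPlay copies structure health and armor into StructureDamageComponent, which receives incoming damage along with the causing projectile's critical damage.
; Once IsDestroyed is set, Fracture enables gravity on the Destructible, adjusts its collision responses and applies a radial impulse from just above it.
; Mesh-swap, sound and delayed-destroy nodes are unwired.
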(event `self.ReceiveBeginPlay`
  (bind _structuredamagecomponent (`self.StructureDamageComponent`))
  (set `/Game/MyContent/Blueprints/Components/Damage/MasterDamageComponent_BP.Health` (`self.StructureHealth`) _structuredamagecomponent)
  (set `/Game/MyContent/Blueprints/Components/Damage/MasterDamageComponent_BP.ArmorPercentage` (`self.StructureArmor`) _structuredamagecomponent))

(event `self.ReceiveAnyDamage`
  (params (Damage :type "Float (single-precision)") (DamageType :type "DamageType Object Reference") (InstigatedBy :type "Controller Object Reference") (DamageCauser :type "Actor Object Reference"))
  ;[1 1 1] Comment
  (`/Game/MyContent/Blueprints/Components/Damage/MasterDamageComponent_BP.ReceiveDamage` (`self.StructureDamageComponent`) self Damage (`/Game/MyContent/Blueprints/Projectiles/MasterProjectile_BP.CriticalDamage` (cast `/Game/MyContent/Blueprints/Projectiles/MasterProjectile_BP` DamageCauser :!pure true)))
  (if (`self.IsDestroyed`)
    (`self.Fracture`)))

(event `Fracture`
  (bind (_returnvalue_x _returnvalue_y _returnvalue_z) (`KismetMathLibrary.BreakVector` (`SceneComponent.K2_GetComponentLocation` (`self.Destructible`))))
  ;[1 1 1] Set Fracture objects Collision Responder and Make a Sound on destruction
  (`KismetSystemLibrary.PrintString` "Fracture")
  (`PrimitiveComponent.SetEnableGravity` (`self.Destructible`) true)
  (`PrimitiveComponent.SetCollisionResponseToChannel` (`self.Destructible`) "ECC_PhysicsBody" "ECR_Ignore")
  (`PrimitiveComponent.SetCollisionResponseToChannel` (`self.Destructible`) "ECC_Destructible" "ECR_Block")
  (`PrimitiveComponent.SetCollisionResponseToChannel` (`self.Destructible`) "ECC_WorldStatic" "ECR_Block")
  (`PrimitiveComponent.AddRadialImpulse` (`self.Destructible`) (`KismetMathLibrary.MakeVector` _returnvalue_x _returnvalue_y (+ _returnvalue_z 50.0)) 500.0 100.0 "RIF_Constant" false))

(event `self.Destructible.OnComponentFracture`
  (params (HitPoint :type "Vector Structure (by ref)") (HitDirection :type "Vector Structure (by ref)")))

(fn `UserConstructionScript`)